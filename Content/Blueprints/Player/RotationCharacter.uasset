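; Player character Blueprint for a shooter, handling two guns, bullet damage, minimap resizing, pause menu and upgrade screen.
; The MainPlayerHud widget it creates stores health, ammo and gun selection; bullet_basic hits drain health until the actor is destroyed.
; Shooting uses a gated delay for fire rate, while reload and gun switch block fire during a stepped HUD countdown scaled by QuickHandTime, then refill ammo.
; Tick manually updates every Minimicam actor.
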(event `Key|U`
  (params (Key :type "Key Structure" :default "AnyKey"))
  (bind _returnvalue (`GameplayStatics.GetPlayerController` 0))
  (bind _returnvalue_2 (`GameplayStatics.GetPlayerController` 0))
  (bind _upgrade_screen (`self.Upgrade Screen`))
  (:`Pressed`
    (`/Engine/EditorBlueprintResources/StandardMacros.FlipFlop`
      (:`A`
        (bind _returnvalue_3 (`|CreateWidget` "/Game/Blueprints/Ui/UpgradeScreen.UpgradeScreen_C"))
        (set `self.Upgrade Screen` _returnvalue_3)
        (`WidgetBlueprintLibrary.SetInputMode_GameAndUIEx` _returnvalue_2 _upgrade_screen)
        (`UserWidget.AddToViewport` _upgrade_screen 0)
        (set `PlayerController.bShowMouseCursor` true _returnvalue_2))
      (:`B`
        (`WidgetBlueprintLibrary.SetInputMode_GameAndUIEx` _returnvalue)
        (set `PlayerController.bShowMouseCursor` false _returnvalue)
        (`Widget.RemoveFromParent` _returnvalue_3)
        (`GameplayStatics.SetGamePaused` false)))))

(event `self.ReceiveTick`
  (params (DeltaSeconds :type "Float (single-precision)"))
  ;[1 1 1] Drawminimap
  (bind _outactors (`GameplayStatics.GetAllActorsOfClass` "/Game/Blueprints/Minimap/Minimicam.Minimicam_C"))
  (for _array_element _outactors
    (`/Game/Blueprints/Minimap/Minimicam.OutSideTick` _array_element)))

(event `self.ReceiveBeginPlay`
  (bind _mainplayerhudref (`self.MainPlayerHUDRef`))
  ;[1 1 1] initialize
  (bind _returnvalue (`|CreateWidget` "/Game/Blueprints/Ui/mainPlayerHud.mainPlayerHud_C" (`GameplayStatics.GetPlayerController` 0)))
  (bind _output_get (set `self.MainPlayerHUDRef` _returnvalue))
  (`UserWidget.AddToViewport` _output_get 0)
  (set `/Game/Blueprints/Ui/mainPlayerHud.Health` 100.0 _mainplayerhudref)
  (set `/Game/Blueprints/Ui/mainPlayerHud.mana` 100.0 _mainplayerhudref)
  (`WidgetBlueprintLibrary.SetInputMode_GameOnly` (`GameplayStatics.GetPlayerController` 0)))

(event `self.CapsuleComponent.OnComponentHit`
  (params (HitComponent :type "PrimitiveComponent Object Reference") (OtherActor :type "Actor Object Reference") (OtherComp :type "PrimitiveComponent Object Reference") (NormalImpulse :type "Vector Structure") (Hit :type "HitResult Structure (by ref)"))
  (cast `/Game/Blueprints/Actors/Bullets/bullet_basic` OtherActor)
  (set `/Game/Blueprints/Ui/mainPlayerHud.Health` (- (`/Game/Blueprints/Ui/mainPlayerHud.Health` (`self.MainPlayerHUDRef`)) 5.0) (`self.MainPlayerHUDRef`))
  (`self.K2_DestroyActor` OtherActor)
  (`self.EnemyHit`))

(event `InputAction|Enlargeminimap`
  (params (Key :type "Key Structure" :default "AnyKey"))
  (:`Pressed`
    (if (`self.MinimapSizeup`)
      (`/Engine/EditorBlueprintResources/StandardMacros.FlipFlop`
        (:`A`
          (`self.Minimap SUp `))
        (:`B`
          (`self.Minimap SDown`)))
      (`KismetSystemLibrary.Delay` 1.5)
      (set `self.MinimapSizeup` true))))

(event `EnemyHit`
  (if (>= 0.0 (`/Game/Blueprints/Ui/mainPlayerHud.Health` (`self.MainPlayerHUDRef`)))
    (`self.K2_DestroyActor`)))

(event `InputAction|Shoot`
  (params (Key :type "Key Structure" :default "AnyKey"))
  (bind _mainplayerhudref (`self.MainPlayerHUDRef`))
  (bind _basicpistol (`/Game/Blueprints/Ui/mainPlayerHud.basicpistol` _mainplayerhudref))
  ;[1 1 1] PlayerShooting
  (:`Pressed`
    (if (`self.Disableshooting`)
      _
      (elif (== _basicpistol 0.0)
        (`GameplayStatics.PlaySoundAtLocation` "/Game/Audio/GameSounds/clp.clp")
        (elif (>= _basicpistol 0.0)
          (`/Engine/EditorBlueprintResources/StandardMacros.Gate` false :!label _label
            (:`Exit`
              (`|ExecutionSequence`
                (:`then_0`
                  (bind _currentusedgun (`self.GetgunInUse` (`/Game/Blueprints/Ui/mainPlayerHud.MainOfHand` _mainplayerhudref)))
                  (`self.FireProjectile` _currentusedgun)
                  (set `/Game/Blueprints/Ui/mainPlayerHud.basicpistol` (- (`/Game/Blueprints/Ui/mainPlayerHud.basicpistol` _mainplayerhudref) 1.0) _mainplayerhudref)
                  (`KismetSystemLibrary.Delay` (`self.GunshotDelay`))
                  (goto _label :!via `Open`))
                (:`then_1`
                  (goto _label :!via `Close`))))))))))

(event `InputAction|Pause`
  (params (Key :type "Key Structure" :default "AnyKey"))
  (bind _returnvalue (`GameplayStatics.GetPlayerController` 0))
  (bind _pausemenuref (`self.PauseMenuRef`))
  (:`Pressed`
    (`/Engine/EditorBlueprintResources/StandardMacros.IsValid` (`self.PauseMenuRef`)
      (:`Is Valid`
        _)
      (:`Is Not Valid`
        (bind _returnvalue_2 (`|CreateWidget` "/Game/Blueprints/Ui/IngameMenu.IngameMenu_C"))
        (set `self.PauseMenuRef` _returnvalue_2)))
    (`WidgetBlueprintLibrary.SetInputMode_UIOnlyEx` _returnvalue _pausemenuref)
    (`UserWidget.AddToViewport` _pausemenuref 0)
    (`GameplayStatics.SetGamePaused` true)
    (set `PlayerController.bShowMouseCursor` true _returnvalue)))

(event `InputAction|switchgun`
  (params (Key :type "Key Structure" :default "AnyKey"))
  (:`Pressed`
    (`self.SwitchGun`)))

(event `InputAction|reload`
  (params (Key :type "Key Structure" :default "AnyKey"))
  (:`Pressed`
    (`self.ReloadTime`)))

(fn `FireProjectile`
  (params (GetBullet :type "Actor Class Reference"))
  (`|SpawnActorFromClass` GetBullet (`SceneComponent.K2_GetComponentToWorld` (`self.Arrow1`)) "AdjustIfPossibleButAlwaysSpawn" "OverrideRootScale")
  (`GameplayStatics.PlaySoundAtLocation` (`self.Sound+`)))

(fn `GetgunInUse`
  (params (Condition :type Boolean))
  (returns (CurrentUsedGun :type "Actor Class Reference"))
  (if Condition
    (set `self.CurrentUsedGun` "/Game/Blueprints/Actors/Bullets/bullet_basic2.bullet_basic2_C")
    (set `self.Sound+` "/Game/Audio/GameSounds/M1_Garand_Single-SoundBible_com-1941178963.M1_Garand_Single-SoundBible_com-1941178963")
    (set `self.GunshotDelay` 0.2)
    (else
      (set `self.CurrentUsedGun` "/Game/Blueprints/Actors/Bullets/bullet_basic.bullet_basic_C")
      (set `self.Sound+` "/Game/Audio/GameSounds/revolver.revolver")
      (set `self.GunshotDelay` 0.5)))
  (return (`self.CurrentUsedGun`)))

(fn `GetHIT`
  (params (NewParam :type "/Game/Blueprints/Actors/Bullets/BulletGeneric Object Reference")))

(fn `Minimap SDown`
  (bind _mainplayerhudref (`self.MainPlayerHUDRef`))
  (`UserWidget.PlayAnimation` _mainplayerhudref (`/Game/Blueprints/Ui/mainPlayerHud.sizedown` _mainplayerhudref) 0.0 1 "Forward" 1.0)
  (set `self.MinimapSizeup` false)
  (return))

(fn `Minimap SUp `
  (bind _mainplayerhudref (`self.MainPlayerHUDRef`))
  (`UserWidget.PlayAnimation` _mainplayerhudref (`/Game/Blueprints/Ui/mainPlayerHud.sizeup` _mainplayerhudref) 0.0 1 "Forward" 1.0)
  (set `self.MinimapSizeup` false)
  (return))

(fn `NewFunction_0`
  (params (Condition :type Boolean) (self2 :type "/Game/Blueprints/Ui/mainPlayerHud Object Reference")))

(fn `UserConstructionScript`)