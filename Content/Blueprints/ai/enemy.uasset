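; Enemy actor for a top-down shooter that takes bullet damage, fires back and awards score when killed.
; Capsule hits from bullet_basic reduce BaseHealth, destroy the bullet, update the Aihealth widget's progress bar and run EnemyHit.
; At zero health, EnemyHit destroys the enemy and adds score to the player's TopDownCharacter.
; Each Box overlap, after a short delay, spawns one bullet at a yaw-offset point with a gunshot sound.
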(event `self.CapsuleComponent.OnComponentHit`
  (params (HitComponent :type "PrimitiveComponent Object Reference") (OtherActor :type "Actor Object Reference") (OtherComp :type "PrimitiveComponent Object Reference") (NormalImpulse :type "Vector Structure") (Hit :type "HitResult Structure (by ref)"))
  (cast `/Game/Blueprints/Actors/Bullets/bullet_basic` OtherActor)
  (set `self.BaseHealth` (- (`self.BaseHealth`) 20.0))
  (`self.K2_DestroyActor` OtherActor)
  (bind _asaihealth (cast `/Game/Blueprints/Ui/Aihealth` (`WidgetComponent.GetUserWidgetObject` (`self.Widget`))))
  (`ProgressBar.SetPercent` (`/Game/Blueprints/Ui/Aihealth.ProgressBar_50` _asaihealth) (/ (`self.BaseHealth`) 100.0))
  (`self.EnemyHit`))

(event `EnemyHit`
  (if (>= 0.0 (`self.BaseHealth`))
    (`self.K2_DestroyActor`)
    (bind _astop_down_character (cast `/Game/Blueprints/TopDownCharacter` (`GameplayStatics.GetPlayerCharacter` 0)))
    (set `/Game/Blueprints/TopDownCharacter.score` (+ (`/Game/Blueprints/TopDownCharacter.score` _astop_down_character) 100.0) _astop_down_character)))

(event `self.Box.OnComponentBeginOverlap`
  (params (OverlappedComponent :type "PrimitiveComponent Object Reference") (OtherActor :type "Actor Object Reference") (OtherComp :type "PrimitiveComponent Object Reference") (OtherBodyIndex :type Integer) (bFromSweep :type Boolean) (SweepResult :type "HitResult Structure (by ref)"))
  (bind _returnvalue (+ (.yaw (`self.K2_GetActorRotation`)) 35.0))
  (`KismetSystemLibrary.Delay` 0.2)
  (`|SpawnActorFromClass` "/Game/Blueprints/Actors/Bullets/bullet_basic.bullet_basic_C" (`KismetMathLibrary.MakeTransform` (`KismetMathLibrary.MakeVector` (+ (.x (`self.K2_GetActorLocation`)) (* (`KismetMathLibrary.DegCos` _returnvalue) 75.0)) (+ (.y (`self.K2_GetActorLocation`)) (* (`KismetMathLibrary.DegSin` _returnvalue) 75.0)) (.z (`self.K2_GetActorLocation`))) (`self.K2_GetActorRotation`) (0.5 0.5 0.5)) "AdjustIfPossibleButDontSpawnIfColliding" "OverrideRootScale")
  (`GameplayStatics.PlaySoundAtLocation` "/Game/Audio/GameSounds/M1_Garand_Single-SoundBible_com-1941178963.M1_Garand_Single-SoundBible_com-1941178963" (`self.K2_GetActorLocation`)))

(fn `UserConstructionScript`)