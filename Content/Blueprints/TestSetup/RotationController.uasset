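; RotationController is a test-setup controller for moving its pawn and turning it toward the mouse cursor.
; MoveForward and MoveRight axis inputs push the controlled pawn along fixed world X and Y, independent of its facing.
; Every tick it sets the pawn's yaw from a look-at toward the deprojected mouse world location, zeroing pitch and roll.
; The aim uses that deprojected point directly, with no trace or hit test.
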(event `InputAxis|MoveForward`
  (params (AxisValue :type "Float (single-precision)"))
  ;[1 1 1] Input Movemnt WASD/CONTROLLER
  (`Pawn.AddMovementInput` (`self.K2_GetPawn`) (1.0 0.0 0.0) AxisValue false))

(event `self.ReceiveTick`
  (params (DeltaSeconds :type "Float (single-precision)"))
  (bind _returnvalue (`self.K2_GetPawn`))
  ;[1 1 1] Get Hit RegistrationUnderMouseCursor
  (`self.K2_SetActorRotation` _returnvalue (`KismetMathLibrary.MakeRotator` 0.0 0.0 (.yaw (`KismetMathLibrary.FindLookAtRotation` (`self.K2_GetActorLocation` _returnvalue) (`self.DeprojectMousePositionToWorld`)))) false))

(event `InputAxis|MoveRight`
  (params (AxisValue :type "Float (single-precision)"))
  ;[1 1 1] Input Movemnt WASD/CONTROLLER
  (`Pawn.AddMovementInput` (`self.K2_GetPawn`) (0.0 1.0 0.0) AxisValue false))

(fn `UserConstructionScript`)