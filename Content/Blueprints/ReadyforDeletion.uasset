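; Top-down shooter player character that moves on world axes, turns toward the cursor and fires bullets from an offset transform.
; The MainPlayerHud widget created at BeginPlay holds health, ammo and weapon selection, with bullet hits draining health until the actor is destroyed.
; Reload and gun switch refill ammo through delayed countdown steps.
; Keys open upgrade and pause menus or resize the HUD, and Tick updates every Minimicam through GetAllActorsOfClass.
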(event `Key|U`
  (params (Key :type "Key Structure" :default "AnyKey"))
  (bind _returnvalue (`GameplayStatics.GetPlayerController` 0))
  (bind _upgrade_screen (`self.Upgrade Screen`))
  ;[0.46 0 0.03843] Comment
  (:`Pressed`
    (`/Engine/EditorBlueprintResources/StandardMacros.FlipFlop`
      (:`A`
        (bind _returnvalue_2 (`|CreateWidget` "/Game/Blueprints/Ui/UpgradeScreen.UpgradeScreen_C"))
        (set `self.Upgrade Screen` _returnvalue_2)
        (`WidgetBlueprintLibrary.SetInputMode_UIOnlyEx` _returnvalue _upgrade_screen)
        (`UserWidget.AddToViewport` _upgrade_screen 0)
        (`GameplayStatics.SetGamePaused` true)
        (set `PlayerController.bShowMouseCursor` true _returnvalue)))))

(event `Key|M`
  (params (Key :type "Key Structure" :default "AnyKey"))
  (bind _mainplayerhud (`self.MainPlayerHud`))
  ;[0.46 0 0.03843] Comment
  (:`Pressed`
    (if (`self.Waitforanimationtoplay`)
      (`/Engine/EditorBlueprintResources/StandardMacros.FlipFlop`
        (:`A`
          (`UserWidget.PlayAnimation` _mainplayerhud (`/Game/Blueprints/Ui/mainPlayerHud.sizeup` _mainplayerhud) 0.0 1 "Forward" 1.0)
          (set `self.Waitforanimationtoplay` false)
          (`KismetSystemLibrary.Delay` 1.5)
          (set `self.Waitforanimationtoplay` true))
        (:`B`
          (`UserWidget.PlayAnimation` _mainplayerhud (`/Game/Blueprints/Ui/mainPlayerHud.sizedown` _mainplayerhud) 0.0 1 "Forward" 1.0)
          (set `self.Waitforanimationtoplay` false)
          (`KismetSystemLibrary.Delay` 1.5)
          (set `self.Waitforanimationtoplay` true))))))

(event `Key|P`
  (params (Key :type "Key Structure" :default "AnyKey"))
  (bind _returnvalue (`GameplayStatics.GetPlayerController` 0))
  (bind _pausemenuref (`self.PauseMenuRef`))
  ;[0.46 0 0.03843] Comment
  (:`Pressed`
    (`/Engine/EditorBlueprintResources/StandardMacros.IsValid` (`self.PauseMenuRef`)
      (:`Is Valid`
        _)
      (:`Is Not Valid`
        (bind _returnvalue_2 (`|CreateWidget` "/Game/Blueprints/Ui/IngameMenu.IngameMenu_C"))
        (set `self.PauseMenuRef` _returnvalue_2)))
    (`WidgetBlueprintLibrary.SetInputMode_UIOnlyEx` _returnvalue _pausemenuref)
    (`UserWidget.AddToViewport` _pausemenuref 0)
    (`GameplayStatics.SetGamePaused` true)
    (set `PlayerController.bShowMouseCursor` true _returnvalue)))

(event `self.ReceiveTick`
  (params (DeltaSeconds :type "Float (single-precision)"))
  ;[0.46 0 0.03843] Comment
  (bind _outactors (`GameplayStatics.GetAllActorsOfClass` "/Game/Blueprints/Minimap/Minimicam.Minimicam_C"))
  (for _array_element _outactors
    (`/Game/Blueprints/Minimap/Minimicam.OutSideTick` _array_element)))

(event `InputAxis|MoveForward`
  (params (AxisValue :type "Float (single-precision)"))
  ;[0 1 0] BASIC Movement
  (`self.AddMovementInput` (1.0 0.0 0.0) AxisValue))

(event `Key|X`
  (params (Key :type "Key Structure" :default "AnyKey"))
  ;[0.46 0 0.03843] Comment
  (:`Pressed`
    (`/Engine/EditorBlueprintResources/StandardMacros.FlipFlop`
      (:`A`
        (set `/Game/Blueprints/Ui/mainPlayerHud.wichisselected` true (`self.MainPlayerHud`)))
      (:`B`
        (set `/Game/Blueprints/Ui/mainPlayerHud.wichisselected` false (`self.MainPlayerHud`))))))

(event `InputAxis|MoveRight`
  (params (AxisValue :type "Float (single-precision)"))
  ;[0 1 0] BASIC Movement
  (`self.AddMovementInput` (0.0 1.0 0.0) AxisValue))

(event `Key|LeftMouseButton`
  (params (Key :type "Key Structure" :default "AnyKey"))
  (bind _returnvalue (`self.K2_GetActorLocation` (`GameplayStatics.GetPlayerController` 0)))
  (bind _returnvalue_2 (`self.ShootLeftHand` (`self.K2_GetActorLocation`) (`self.K2_GetActorRotation`)))
  (bind _basicpistol (`/Game/Blueprints/Ui/mainPlayerHud.basicpistol` (`self.MainPlayerHud`)))
  (bind _mainofhand (`/Game/Blueprints/Ui/mainPlayerHud.MainOfHand` (`self.MainPlayerHud`)))
  ;[1 1 1] Shooting
  (:`Pressed`
    (if (`self.Disableshooting`)
      _
      (elif (== _basicpistol 0.0)
        _
        (elif (>= _basicpistol 0.0)
          (bind (_offhand _mainhand) (`self.GetGunInUse` _mainofhand))
          (if _mainofhand
            (`KismetSystemLibrary.Delay` 0.5)
            (`|SpawnActorFromClass` _offhand _returnvalue_2 "AlwaysSpawn" "OverrideRootScale")
            (`GameplayStatics.PlaySoundAtLocation` "/Game/Audio/GameSounds/revolver.revolver" _returnvalue)
            (else
              (`KismetSystemLibrary.Delay` 0.25)
              (`|SpawnActorFromClass` _mainhand _returnvalue_2 "AlwaysSpawn" "OverrideRootScale")
              (`GameplayStatics.PlaySoundAtLocation` "/Game/Audio/GameSounds/M1_Garand_Single-SoundBible_com-1941178963.M1_Garand_Single-SoundBible_com-1941178963" _returnvalue)))
          (set `/Game/Blueprints/Ui/mainPlayerHud.basicpistol` (- (`/Game/Blueprints/Ui/mainPlayerHud.basicpistol` (`self.MainPlayerHud`)) 1.0) (`self.MainPlayerHud`)))))))

(event `self.ReceiveBeginPlay`
  ;[0.46 0 0.03843] Respawn
  (bind _returnvalue (`|CreateWidget` "/Game/Blueprints/Ui/mainPlayerHud.mainPlayerHud_C" (`GameplayStatics.GetPlayerController` 0)))
  (bind _output_get (set `self.MainPlayerHud` _returnvalue))
  (`UserWidget.AddToViewport` _output_get 0)
  (set `/Game/Blueprints/Ui/mainPlayerHud.Health` 100.0 (`self.MainPlayerHud`))
  (set `/Game/Blueprints/Ui/mainPlayerHud.mana` 100.0 (`self.MainPlayerHud`))
  (`WidgetBlueprintLibrary.SetInputMode_GameOnly` (`GameplayStatics.GetPlayerController` 0)))

(event `self.CapsuleComponent.OnComponentHit`
  (params (HitComponent :type "PrimitiveComponent Object Reference") (OtherActor :type "Actor Object Reference") (OtherComp :type "PrimitiveComponent Object Reference") (NormalImpulse :type "Vector Structure") (Hit :type "HitResult Structure (by ref)"))
  ;[0.46 0 0.03843] DamageApplyed
  (cast `/Game/Blueprints/Actors/Bullets/bullet_basic` OtherActor)
  (set `/Game/Blueprints/Ui/mainPlayerHud.Health` (- (`/Game/Blueprints/Ui/mainPlayerHud.Health` (`self.MainPlayerHud`)) 5.0) (`self.MainPlayerHud`))
  (`self.K2_DestroyActor` OtherActor)
  (`self.EnemyHit`))

(event `InputAxis|LookupM`
  (params (AxisValue :type "Float (single-precision)"))
  ;[0.46 0 0.03843] Look
  (if (not (`self.InputMode`)) :!label _label
    (`self.K2_SetActorRotation` (`KismetMathLibrary.MakeRotator` 0.0 0.0 (.yaw (`KismetMathLibrary.FindLookAtRotation` (`self.K2_GetActorLocation`) (`.Location` (`GameplayStatics.BreakHitResult` (`PlayerController.GetHitResultUnderCursorByChannel` (`GameplayStatics.GetPlayerController` 0) "TraceTypeQuery1" true)))))))))

(event `InputAxis|lookrightM`
  (params (AxisValue :type "Float (single-precision)"))
  ;[0.46 0 0.03843] Look
  (goto _label))

(event `EnemyHit`
  ;[0.46 0 0.03843] Comment
  (if (>= 0.0 (`/Game/Blueprints/Ui/mainPlayerHud.Health` (`self.MainPlayerHud`)))
    (`self.K2_DestroyActor`)))

(event `InputAxis|LookupC`
  (params (AxisValue :type "Float (single-precision)"))
  ;[0.46 0 0.03843] Comment
  (bind _returnvalue (`KismetMathLibrary.MakeVector` AxisValue (stale `InputAxis|lookrightC` AxisValue)))
  (if (> (`KismetMathLibrary.VSize` _returnvalue) 0.25) :!label _label_2
    (`Controller.SetControlRotation` (`GameplayStatics.GetPlayerController` 0) (`KismetMathLibrary.Conv_VectorToRotator` _returnvalue))))

(event `InputAction|reload`
  (params (Key :type "Key Structure" :default "AnyKey"))
  (bind _mainplayerhud (`self.MainPlayerHud`))
  ;[0.46 0 0.03843] Comment
  (:`Pressed`
    (set `/Game/Blueprints/Ui/mainPlayerHud.Ros` true _mainplayerhud)
    (if (not (`/Game/Blueprints/Ui/mainPlayerHud.Startcountdown` _mainplayerhud))
      (set `/Game/Blueprints/Ui/mainPlayerHud.Startcountdown` true _mainplayerhud)
      (set `/Game/Blueprints/Ui/mainPlayerHud.getpercent` 100.0 _mainplayerhud)
      (`KismetSystemLibrary.Delay` 0.5)
      (set `/Game/Blueprints/Ui/mainPlayerHud.getpercent` 80.0 _mainplayerhud)
      (`KismetSystemLibrary.Delay` 0.5)
      (set `/Game/Blueprints/Ui/mainPlayerHud.getpercent` 60.0 _mainplayerhud)
      (`KismetSystemLibrary.Delay` 0.5)
      (set `/Game/Blueprints/Ui/mainPlayerHud.getpercent` 40.0 _mainplayerhud)
      (`KismetSystemLibrary.Delay` 0.5)
      (set `/Game/Blueprints/Ui/mainPlayerHud.getpercent` 20.0 _mainplayerhud)
      (`KismetSystemLibrary.Delay` 0.5)
      (set `/Game/Blueprints/Ui/mainPlayerHud.basicpistol` 12.0 _mainplayerhud)
      (set `/Game/Blueprints/Ui/mainPlayerHud.Startcountdown` false _mainplayerhud))))

(event `InputAxis|lookrightC`
  (params (AxisValue :type "Float (single-precision)"))
  ;[0.46 0 0.03843] Comment
  (goto _label_2))

(event `InputAction|switchgun`
  (params (Key :type "Key Structure" :default "AnyKey"))
  (bind _mainplayerhud (`self.MainPlayerHud`))
  (:`Pressed`
    (set `/Game/Blueprints/Ui/mainPlayerHud.Ros` false _mainplayerhud)
    (if (not (`/Game/Blueprints/Ui/mainPlayerHud.Startcountdown` _mainplayerhud))
      (set `self.Disableshooting` true)
      (set `/Game/Blueprints/Ui/mainPlayerHud.Startcountdown` true _mainplayerhud)
      (set `/Game/Blueprints/Ui/mainPlayerHud.getpercent` 100.0 _mainplayerhud)
      (`KismetSystemLibrary.Delay` 0.5)
      (set `/Game/Blueprints/Ui/mainPlayerHud.getpercent` 80.0 _mainplayerhud)
      (`KismetSystemLibrary.Delay` 0.5)
      (set `/Game/Blueprints/Ui/mainPlayerHud.getpercent` 60.0 _mainplayerhud)
      (`KismetSystemLibrary.Delay` 0.5)
      (set `/Game/Blueprints/Ui/mainPlayerHud.getpercent` 40.0 _mainplayerhud)
      (`KismetSystemLibrary.Delay` 0.5)
      (set `/Game/Blueprints/Ui/mainPlayerHud.getpercent` 20.0 _mainplayerhud)
      (`KismetSystemLibrary.Delay` 0.5)
      (set `/Game/Blueprints/Ui/mainPlayerHud.basicpistol` 12.0 _mainplayerhud)
      (set `/Game/Blueprints/Ui/mainPlayerHud.Startcountdown` false _mainplayerhud)
      (`/Engine/EditorBlueprintResources/StandardMacros.FlipFlop`
        (:`A`
          (set `/Game/Blueprints/Ui/mainPlayerHud.wichisselected` false (`self.MainPlayerHud`)))
        (:`B`
          (set `/Game/Blueprints/Ui/mainPlayerHud.wichisselected` true (`self.MainPlayerHud`))))
      (set `self.Disableshooting` false))))

(fn `Cast from Hudref`
  (returns (MainPlayerHUD :type "/Game/Blueprints/Ui/mainPlayerHud Object Reference")))

(fn `Cast from MainGamemode`
  (returns (GameModeRef :type "/Game/Blueprints/GameMode/ThirdPersonGameMode Object Reference"))
  (bind _asthird_person_game_mode (cast `/Game/Blueprints/GameMode/ThirdPersonGameMode` (`GameplayStatics.GetGameMode`)))
  (return _asthird_person_game_mode))

(fn `GetGunInUse`
  (params (NewParam :type Boolean))
  (returns (OffHand :type "Actor Class Reference") (Mainhand :type "Actor Class Reference"))
  (if NewParam
    (set `self.CurrentlyUsedGunoffHand` "/Game/Blueprints/Actors/Bullets/bullet_basic.bullet_basic_C")
    (else
      (set `self.CurrentlyUsedGunmainHand` "/Game/Blueprints/Actors/Bullets/bullet_basic2.bullet_basic2_C")))
  (return (`self.CurrentlyUsedGunoffHand`) (`self.CurrentlyUsedGunmainHand`)))

(fn `ShootLeftHand`
  (params (InVec :type "Vector Structure") (InRot :type "Rotator Structure"))
  (returns (ReturnValue :type "Transform Structure"))
  (bind _returnvalue (+ (.yaw InRot) 35.0))
  (return (`KismetMathLibrary.MakeTransform` (`KismetMathLibrary.MakeVector` (+ (.x InVec) (* (`KismetMathLibrary.DegCos` _returnvalue) 100.0)) (+ (.y InVec) (* (`KismetMathLibrary.DegSin` _returnvalue) 100.0)) (.z InVec)) (`self.K2_GetActorRotation`) (0.4 0.4 0.4))))

(fn `ShootRightHand`
  (params (InVec :type "Vector Structure") (InRot :type "Rotator Structure"))
  (returns (ReturnValue :type "Transform Structure"))
  (bind _returnvalue (+ (.yaw InRot) -35.0))
  (return (`KismetMathLibrary.MakeTransform` (`KismetMathLibrary.MakeVector` (+ (.x InVec) (* (`KismetMathLibrary.DegCos` _returnvalue) 100.0)) (+ (.y InVec) (* (`KismetMathLibrary.DegSin` _returnvalue) 100.0)) (.z InVec)) (`self.K2_GetActorRotation`) (0.4 0.4 0.4))))

(fn `UserConstructionScript`)